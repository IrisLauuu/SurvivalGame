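; GlobalTimer is a day/night clock actor that turns game time into sun position and calendar values.
; Each Tick, it pitches SunLight by elapsed day fraction, scaled by SecondsPerDay, and refreshes the SkySphere sun direction.
; It derives CurrentDay, CurrentHour and CurrentMin through chained whole-and-remainder divisions, then sets IsDayTime from the hour.
; A gate, open by default, guards these updates until StopTimer closes it, with no reopen path here.
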(event Custom|StopTimer
  (bind _returnvalue (Utilities|Time|GetGameTimeinSeconds))
  (bind _secondsperday (Variables|Default|GetSecondsPerDay))
  (bind (_remainder _returnvalue_2) (Math|Float|Division(WholeandRemainder) _returnvalue _secondsperday))
  (bind _returnvalue_3 (/ _secondsperday 24.0))
  (bind (_remainder_2 _returnvalue_4) (Math|Float|Division(WholeandRemainder) _remainder _returnvalue_3))
  (Utilities|FlowControl|Gate false) ; enters at Close
)

(event EventBeginPlay)

(event Collision|EventActorBeginOverlap
  (params (OtherActor :type Actor%20Object%20Reference)))

(event EventTick
  (params (DeltaSeconds :type Float%20%28single-precision%29))
  (bind _returnvalue (Utilities|Time|GetGameTimeinSeconds))
  (bind _secondsperday (Variables|Default|GetSecondsPerDay))
  (bind (_remainder _returnvalue_2) (Math|Float|Division(WholeandRemainder) _returnvalue _secondsperday))
  (bind _returnvalue_3 (/ _secondsperday 24.0))
  (bind (_remainder_2 _returnvalue_4) (Math|Float|Division(WholeandRemainder) _remainder _returnvalue_3))
  (Utilities|FlowControl|Gate false
    (:Exit
      (Transformation|SetActorRotation (Variables|Default|GetSunLight) (Math|Rotator|MakeRotator 0.0 (+ (* (/ _remainder _secondsperday) 3.6e+02) -9e+01) 0.0))
      (Default|UpdateSunDirection (Variables|Default|GetSkySphere))
      (Variables|Default|SetCurrentDay _returnvalue_2)
      (bind _output_get (Variables|Default|SetCurrentHour _returnvalue_4))
      (Variables|Default|SetCurrentMin (.ReturnValue (Math|Float|Division(WholeandRemainder) _remainder_2 (/ _returnvalue_3 6e+01))))
      (Variables|Default|SetIsDayTime (Math|Integer|InRange(Integer) _output_get 6 18 true false)))))

(fn ConstructionScript)