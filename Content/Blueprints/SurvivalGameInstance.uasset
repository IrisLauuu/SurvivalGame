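; Game instance for a survival game that owns and controls the runtime UI and pickup panel widgets.
; CreateRuntimeUI lazily creates the runtime UI once and adds it to the viewport.
; CreatePickUpUI creates or reuses the cached pickable panel, shows it, and switches to game-and-UI input with a visible cursor.
; HidePickablePanel removes the panel, keeping its reference, and restores game-only input with a hidden cursor.
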(event Custom|CreateRuntimeUI
  (Utilities|IsValid (Variables|Default|GetRuntimeUI)
    (:Is%20Not%20Valid
      (bind _returnvalue (UserInterface|CreateWidget "/Game/UI/UI_RuntimeUI.UI_RuntimeUI_C" (Game|GetPlayerController 0)))
      (bind _output_get (Variables|Default|SetRuntimeUI _returnvalue))
      (UserInterface|Viewport|AddtoViewport _output_get 0))))

(event Custom|CreatePickUpUI
  (bind _returnvalue (Game|GetPlayerController 0))
  (Utilities|IsValid (Variables|Default|GetPickableUI)
    (:Is%20Valid
      (if (not (UserInterface|Viewport|IsinViewport (Variables|Default|GetPickableUI)))
        (UserInterface|Viewport|AddtoViewport (stale _output_get) 0 :!label _label)
        (Input|SetInputModeGameandUI _returnvalue (Variables|Default|GetPickableUI) "DoNotLock" true)
        (Variables|/Script/Engine.PlayerController|SetbShowMouseCursor _returnvalue true)))
    (:Is%20Not%20Valid
      (bind _returnvalue_2 (UserInterface|CreateWidget "/Game/UI/UI_PickablePanel.UI_PickablePanel_C" (Game|GetPlayerController 0)))
      (bind _output_get (Variables|Default|SetPickableUI _returnvalue_2))
      (goto _label))))

(event Custom|HidePickablePanel
  (bind _returnvalue (Game|GetPlayerController 0))
  (bind _pickableui (Variables|Default|GetPickableUI))
  (Utilities|IsValid _pickableui
    (:Is%20Valid
      (Widget|RemovefromParent _pickableui)
      (Input|SetInputModeGameOnly _returnvalue)
      (Variables|/Script/Engine.PlayerController|SetbShowMouseCursor _returnvalue false))))