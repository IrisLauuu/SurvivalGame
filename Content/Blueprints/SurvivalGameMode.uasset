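; SurvivalGameMode is the game mode for a survival game, controlling level startup, game over, restart and exit.
; On BeginPlay it caches the GlobalTimer and StorageBox actors and has the SurvivalGameInstance create the runtime and message UI.
; GameOver stops the timer and swaps all panels for the game-end panel through the game instance.
; Restart reopens MainLevel, and exit runs a console command.
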(event Custom|GameOver
  (bind _survival_game_instance (Variables|Default|GetSurvival%20Game%20Instance))
  (Default|StopTimer (Variables|Default|GetGlobalTimer))
  (Default|HideAllPanels _survival_game_instance)
  (Default|ShowGameEndPanel _survival_game_instance))

(event Custom|GameRestart
  (Game|OpenLevel(byName) "MainLevel"))

(event Custom|ExitGame
  (Development|ExecuteConsoleCommand "Exit" 0))

(event EventBeginPlay
  (bind _outactors (Actor|GetAllActorsOfClass "/Game/Blueprints/GlobalTimer.GlobalTimer_C"))
  (Variables|Default|SetGlobalTimer (Utilities|Array|Get(acopy) _outactors))
  (bind _outactors_2 (Actor|GetAllActorsOfClass "/Game/Blueprints/Items/StorageBox.StorageBox_C"))
  (Variables|Default|SetStorageBox (Utilities|Array|Get(acopy) _outactors_2))
  (bind _output_get (Variables|Default|SetSurvival%20Game%20Instance (.AsSurvival%20Game%20Instance (Utilities|Casting|CastToSurvivalGameInstance (Game|GetGameInstance)))))
  (Default|CreateRuntimeUI _output_get)
  (Default|CreateMessageUI (Variables|Default|GetSurvival%20Game%20Instance)))

(fn ConstructionScript)