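; Inventory Blueprint that adds items to a weight-limited container.
; CheckCapacity multiplies the item type's class-default Weight by its count, adds the current Load and compares the total to Capacity.
; AddItem stores the new load, then merges the count into a slot of matching type or appends a new slot, firing ItemCountChanged or ItemAdded.
; It returns a success flag with feedback text, rejecting items that exceed capacity.
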(fn CheckCapacity
  (params (NewItem :type Item%20Slot%20Structure))
  (bind (_type _name _icon _count) (Utilities|Struct|BreakItemSlot NewItem))
  (bind _load (Variables|Default|GetLoad))
  (bind _weight (Utilities|GetClassDefaults _type))
  (bind _returnvalue (* _weight _count))
  (bind _returnvalue_2 (+ _returnvalue _load))
  (return (<= _returnvalue_2 (Variables|Default|GetCapacity)) _returnvalue_2))

(fn AddItem
  (params (NewItem :type Item%20Slot%20Structure))
  (bind (_type _name _icon _count) (Utilities|Struct|BreakItemSlot NewItem))
  (bind _returnvalue (Utilities|String|Append "Got " _name))
  (bind (_success _newload) (CallFunction|CheckCapacity NewItem))
  (if _success
    (Variables|Default|SetLoad _newload)
    (for (_array_element _array_index) (Variables|Default|GetContent)
      (if (== _type (.Type (Utilities|Struct|BreakItemSlot _array_element)))
        (bind _structout (Utilities|Struct|SetmembersinItemSlot (Utilities|Array|Get(acopy) (Variables|Default|GetContent) _array_index) _type _name _icon (+ _count (.Count (Utilities|Struct|BreakItemSlot _array_element)))))
        (Default|CallItemCountChanged _structout)
        (return true _returnvalue)))
    (Utilities|Array|Add (Variables|Default|GetContent) NewItem)
    (Default|CallItemAdded NewItem)
    (return true _returnvalue)
    (else
      (return false "Inventory is full"))))